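; UserPawn is a VR pawn that sets the tracking origin to floor level on BeginPlay for a standing SteamVR camera.
; Unconnected graph logic would pair the HMD and two Vive trackers through BPTrackingPawnComponent for relative tracking data.
; That inactive chain also sets up UDP communication with an SP7 platform via Tracker0 and attaches to that tracker.
; Tick and the construction script are empty, and a camera transform debug print is also unconnected.
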(event EventBeginPlay
  ;[1 1 1] Set up a Standing Camera for Steam VR
  (Class|HeadMountedDisplayFunctionLibrary|SetTrackingOrigin "Floor"))

(event EventTick
  (params (DeltaSeconds :type Float%20%28single-precision%29)))

(fn ConstructionScript)