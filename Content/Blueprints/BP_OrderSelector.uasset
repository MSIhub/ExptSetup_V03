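; BP_OrderSelector is a keyboard-driven selector for the order in which levels are played.
; Number keys load a preset order, either the pitch, roll, roll-yaw and yaw levels or a placeholder list, with Credits appended, into the custom GameInstance's LevelsOrder.
; S starts the sequence through the GameInstance's NextLevel when an order is set, and R returns to the MainMenu level.
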(event EventBeginPlay
  (bind _asgi_game_instance_custom (Utilities|Casting|CastToGI_GameInstanceCustom (Game|GetGameInstance)))
  (Variables|Default|SetGI _asgi_game_instance_custom))

(event Input|KeyboardEvents|1
  (params (Key :type Key%20Structure))
  ;[1 1 1] Load order  :
  (:Pressed
    (CallFunction|StartCustomlevelOrder (Utilities|Array|MakeArray "Level_Pitch" "Level_Roll" "Level_RollYaw" "Level_Yaw"))))

(event Input|KeyboardEvents|2
  (params (Key :type Key%20Structure))
  ;[1 1 1] Load order :
  (:Pressed
    (CallFunction|StartCustomlevelOrder (Utilities|Array|MakeArray "None" "None"))))

(event Input|KeyboardEvents|S
  (params (Key :type Key%20Structure))
  (bind _gi (Variables|Default|GetGI))
  ;[1 1 1] Press S for starting the game
  (:Pressed
    (if (> (Utilities|Array|Length (Variables|/Game/Blueprints/GI_GameInstanceCustom.GI_GameInstanceCustom_C|GetLevelsOrder _gi)) 0)
      (Default|NextLevel _gi))))

(event Input|KeyboardEvents|R
  (params (Key :type Key%20Structure))
  ;[1 1 1] Press r to reset, come to main menu
  (:Pressed
    (Game|OpenLevel(byName) "MainMenu")))

(fn ConstructionScript)

(fn StartCustomlevelOrder
  (params (LevelOrder :type Array%20of%20Names))
  (Utilities|Array|Add LevelOrder "Credits")
  (Variables|/Game/Blueprints/GI_GameInstanceCustom.GI_GameInstanceCustom_C|SetLevelsOrder (Variables|Default|GetGI) LevelOrder))