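; VR motion-recording Blueprint that logs SteamVR HMD and Vive tracker data for two platforms and the torso.
; Each tick extracts every device's transform and tracker data relative to the initial HMD frame, appending samples to per-device arrays.
; It also derives head-relative-to-torso pose by multiplying the inverse torso matrix with the head matrix, then computes velocity and acceleration.
; EndPlay saves all recorded arrays to text files.
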(event Custom|ExtractTrackerData1
  (params (DeltaSeconds :type Float%20%28single-precision%29))
  ;[1 1 1] Tracker Platform A with respect to HMD(initial0)
  ;;[1 1 1] Extract data from Tracker
  (bind (_gettrackerdatafunc_out _transformationmatrix_wrt_base) (CallFunction|GetTrackerData (Variables|Default|GetTR_PlatformA) DeltaSeconds))
  (Variables|Default|SetTransformation_A_wrt_H0 _transformationmatrix_wrt_base)
  (bind _output_get (Variables|Default|SetTR_PlatformA_TrackerDataStruct _gettrackerdatafunc_out))
  (Utilities|Array|Add (Variables|Default|GetFinal_TR_PlatformA_TrackerDataStruct) _output_get))

(event Custom|SaveData2
  (params (EndPLay%20Reason :type EEndPlayReason%20Enum :default "Destroyed"))
  ;[1 1 1] Tracker Platform B with respect to HMD(initial0)
  ;;[1 1 1] Save Data to Text
  (CallFunction|SaveTrackerDatatxt (Variables|Default|GetFinal_TR_PlatformB_TrackerDataStruct) (Variables|Default|GetFolderName) (Utilities|GetObjectName (Variables|Default|GetTR_PlatformB)) (Variables|Default|GetIsFileOverWriting)))

(event Custom|SaveCalData
  (params (EndPlayReason :type EEndPlayReason%20Enum :default "Destroyed"))
  ;[1 1 1] Save Data to Text
  (CallFunction|SaveTrackerDatatxt (Variables|Default|GetFinal_DataHead_wrt_Torso) (Variables|Default|GetFolderName) "Data Head wrt Torso" (Variables|Default|GetIsFileOverWriting)))

(event Custom|SaveData1
  (params (EndPlayReason :type EEndPlayReason%20Enum :default "Destroyed"))
  ;[1 1 1] Tracker Platform A with respect to HMD(initial0)
  ;;[1 1 1] Save Data to Text
  (CallFunction|SaveTrackerDatatxt (Variables|Default|GetFinal_TR_PlatformA_TrackerDataStruct) (Variables|Default|GetFolderName) (Utilities|GetObjectName (Variables|Default|GetTR_PlatformA)) (Variables|Default|GetIsFileOverWriting)))

(event Custom|ExtractTrackerData3
  (params (DeltaSeconds :type Float%20%28single-precision%29))
  ;[1 1 1] Tracker Torso data with respect to HMD(initial0)
  ;;[1 1 1] Extract data from Tracker of Torso (Vive 2.0)
  (bind (_gettrackerdatafunc_out _transformationmatrix_wrt_base) (CallFunction|GetTrackerData (Variables|Default|GetTR_Torso2_0) DeltaSeconds))
  (Variables|Default|SetTransformation_T_wrt_H0 _transformationmatrix_wrt_base)
  (bind _output_get (Variables|Default|SetTR_Torso2_0_TrackerDataStruct _gettrackerdatafunc_out))
  (Utilities|Array|Add (Variables|Default|GetFinal_TR_Torso2_0_TrackerDataStruct) _output_get))

(event Custom|Cal_Transformation
  (params (DeltaSeconds :type Float%20%28single-precision%29))
  ;[1 1 1] Calculating data of Head with respect to torso
  (bind _returnvalue (Class|TransformationMatrixLib|TransformationMatrixInverse (Variables|Default|GetTransformation_T_wrt_H0)))
  (bind _returnvalue_2 (Class|TransformationMatrixLib|TransformationMatrixMultiply _returnvalue (Variables|Default|GetTransformation_H_wrt_H0)))
  (bind _output_get (Variables|Default|SetTransformation_H_wrt_T _returnvalue_2))
  (bind _returnvalue_3 (Class|TransformationMatrixLib|TransformationMatrixPositionExtract _output_get))
  (bind _returnvalue_4 (Class|TransformationMatrixLib|TransformationMatrixRotationRPYExtract _output_get))
  (bind _gettrackerdatafunc_out (CallFunction|CalVelandAcc _returnvalue_3 _returnvalue_4 DeltaSeconds))
  (bind _output_get_2 (Variables|Default|SetData_Head_wrt_Torso _gettrackerdatafunc_out))
  (Utilities|Array|Add (Variables|Default|GetFinal_DataHead_wrt_Torso) _output_get_2))

(event Custom|SaveData3
  (params (EndPLayReason :type EEndPlayReason%20Enum :default "Destroyed"))
  ;[1 1 1] Tracker Torso data with respect to HMD(initial0)
  ;;[1 1 1] Save Data to txt
  (CallFunction|SaveTrackerDatatxt (Variables|Default|GetFinal_TR_Torso2_0_TrackerDataStruct) (Variables|Default|GetFolderName) (Utilities|GetObjectName (Variables|Default|GetTR_Torso2_0)) (Variables|Default|GetIsFileOverWriting)))

(event Custom|ExtractHMDData
  (params (DeltaSeconds :type Float%20%28single-precision%29))
  ;[1 1 1] HMD Data with respect to HMD(initial0)
  ;;[1 1 1] Extract Data from HMD using steam VR function
  (bind (_outfunctrackerdatastruct _transformationmatrix) (CallFunction|ExtractTrackerData (Variables|Default|GetShowHMDMesh) (Variables|Default|GetHMD) DeltaSeconds "HMD"))
  (Variables|Default|SetTransformation_H_wrt_H0 _transformationmatrix)
  (bind _output_get (Variables|Default|SetHMD_TrackerDataStruct _outfunctrackerdatastruct))
  (Utilities|Array|Add (Variables|Default|GetFinal_HMD_TrackerDataStruct) _output_get))

(event Custom|SaveHMDData
  (params (EndPlayReason :type EEndPlayReason%20Enum :default "Destroyed"))
  ;[1 1 1] HMD Data with respect to HMD(initial0)
  ;;[1 1 1] Save HMD data to txt
  (CallFunction|SaveTrackerDatatxt (Variables|Default|GetFinal_HMD_TrackerDataStruct) (Variables|Default|GetFolderName) "HMD" (Variables|Default|GetIsFileOverWriting)))

(event Custom|ExtractTrackerData2
  (params (DeltaSeconds :type Float%20%28single-precision%29))
  ;[1 1 1] Tracker Platform B with respect to HMD(initial0)
  ;;[1 1 1] Extract data from Tracker and set the static mesh
  (bind (_gettrackerdatafunc_out _transformationmatrix_wrt_base) (CallFunction|GetTrackerData (Variables|Default|GetTR_PlatformB) DeltaSeconds))
  (Variables|Default|SetTransformation_B_wrt_H0 _transformationmatrix_wrt_base)
  (bind _output_get (Variables|Default|SetTR_PlatformB_TrackerDataStruct _gettrackerdatafunc_out))
  (Utilities|Array|Add (Variables|Default|GetFinal_TR_PlatformB_TrackerDataStruct) _output_get))

(event EventBeginPlay
  ;[1 1 1] Set up a Standing Camera for Steam VR
  (Class|HeadMountedDisplayFunctionLibrary|SetTrackingOrigin "Floor"))

(event EventTick
  (params (DeltaSeconds :type Float%20%28single-precision%29))
  (CallFunction|ExtractTrackerData1 DeltaSeconds)
  (CallFunction|ExtractTrackerData2 DeltaSeconds)
  (CallFunction|ExtractTrackerData3 DeltaSeconds)
  (CallFunction|ExtractHMDData DeltaSeconds)
  (CallFunction|CalTransformation DeltaSeconds))

(event EventEndPlay
  (params (EndPlayReason :type EEndPlayReason%20Enum :default "Destroyed"))
  (CallFunction|SaveData1 EndPlayReason)
  (CallFunction|SaveData2 EndPlayReason)
  (CallFunction|SaveData3 EndPlayReason)
  (CallFunction|SaveHMDData EndPlayReason)
  (CallFunction|SaveCalData EndPlayReason))

(fn ConstructionScript)